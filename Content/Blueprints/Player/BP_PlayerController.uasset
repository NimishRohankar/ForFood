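; BP_PlayerController is the player controller that moves the possessed pawn relative to the camera view.
; The Up-Down and Left-Right axis inputs feed AddMovementInput along the camera manager's up and right vectors, after checking that the pawn is valid.
; Using the camera's up vector rather than forward moves the pawn within the screen plane.
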(event EventBeginPlay)

(event EventTick
  (params (DeltaSeconds :type Float%20%28single-precision%29)))

(event Input|AxisEvents|InputAxisUp-Down
  (params (AxisValue :type Float%20%28single-precision%29))
  (bind _returnvalue (Pawn|GetControlledPawn))
  (Utilities|IsValid _returnvalue
    (:Is%20Valid
      (Pawn|Input|AddMovementInput _returnvalue (Math|Vector|GetUpVector (Variables|/Script/Engine.PlayerCameraManager|GetTransformComponent (Variables|Default|GetPlayerCameraManager))) AxisValue false))))

(event Input|AxisEvents|InputAxisLeft-Right
  (params (AxisValue :type Float%20%28single-precision%29))
  (bind _returnvalue (Pawn|GetControlledPawn))
  (Utilities|IsValid _returnvalue
    (:Is%20Valid
      (Pawn|Input|AddMovementInput _returnvalue (Math|Vector|GetRightVector (Variables|/Script/Engine.PlayerCameraManager|GetTransformComponent (Variables|Default|GetPlayerCameraManager))) AxisValue false))))

(fn ConstructionScript)